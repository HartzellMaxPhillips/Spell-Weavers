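; BP_HexShield is a spell actor that gives the player who casts it a temporary shield by lowering their damage multiplier.
; On BeginPlay it plays the shield animation, then pauses it after a short delay to hold that pose.
; It then casts its instigator to PlayerCharacter, sharply reduces DamageMult for ShieldDuration, restores it to normal and destroys itself.
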(event EventBeginPlay
  (Audio|Components|Audio|Play (Variables|Default|GetHexShieldAnim))
  (Utilities|FlowControl|Delay 1.25)
  (Sequencer|Player|Pause (Variables|Default|GetHexShieldAnim))
  (bind _asplayer_character (Utilities|Casting|CastToPlayerCharacter (Game|GetInstigator)))
  (Variables|/Game/ThirdPerson/Blueprints/PlayerCharacter.PlayerCharacter_C|SetDamageMult _asplayer_character 0.1)
  (Utilities|FlowControl|Delay (Variables|Default|GetShieldDuration))
  (Variables|/Game/ThirdPerson/Blueprints/PlayerCharacter.PlayerCharacter_C|SetDamageMult _asplayer_character 1.0)
  (Actor|DestroyActor))

(event Collision|EventActorBeginOverlap
  (params (OtherActor :type Actor%20Object%20Reference)))

(event EventTick
  (params (DeltaSeconds :type Float%20%28single-precision%29)))

(fn ConstructionScript)