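; Fireball spell projectile that, once its Detonated flag is set, stops and becomes a growing, damaging blast.
; Tick drives both the sphere growth, capped by a loop counter, and the detonation sequence; nothing here sets the flag.
; The sequence swaps looping effects, enables the collider after a short delay, then destroys the actor after its lifetime.
; Actors that begin overlapping after detonation take fireball damage.
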(event Custom|Make%20bigger
  (bind _fireballsize (Variables|Default|GetFireballSize))
  (if (and (Variables|Default|GetDetonated) (< (Variables|Default|GetLooptime) 20))
    (Transformation|SetWorldScale3D (Variables|Default|GetSphere) (+ (Transformation|GetWorldScale (Variables|Default|GetSphere)) (Math|Vector|MakeVector _fireballsize _fireballsize _fireballsize)))
    (Variables|Default|SetLooptime (+ (Variables|Default|GetLooptime) 1))
    (Utilities|FlowControl|Delay 0.2)))

(event Custom|Fireball%20Triggered%20Check
  (if (Variables|Default|GetDetonated)
    (Game|Components|ProjectileMovement|SetVelocityinLocalSpace (Variables|Default|GetProjectileMovement) "0, 0, 0")
    (Components|Activation|Activate (Variables|Default|GetFireballLoop2) false)
    (Components|Activation|Deactivate (Variables|Default|GetFireballLoop1))
    (Utilities|FlowControl|Delay 1.0)
    (Components|Activation|Deactivate (Variables|Default|GetFireballLoop2))
    (Components|Activation|Activate (Variables|Default|GetFireballLoop3) true)
    (Collision|SetCollisionEnabled (Variables|Default|GetCollider) "QueryAndPhysics")
    ;[0.15 0.15 0.15 0.5] LIFETIME
    (Utilities|FlowControl|Delay (Variables|Default|GetLifetime))
    (Actor|DestroyActor)))

(event Collision|EventActorBeginOverlap
  (params (OtherActor :type Actor%20Object%20Reference))
  (if (Variables|Default|GetDetonated)
    (Game|Damage|ApplyDamage OtherActor (Variables|Default|GetFireballDamage) 0 0)))

(event EventTick
  (params (DeltaSeconds :type Float%20%28single-precision%29))
  (CallFunction|MakeBigger)
  (CallFunction|FireballTriggeredCheck))

(fn ConstructionScript)